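; Shooter character Blueprint that handles death, kill scoring and the lose screen.
; Tick polls IsDead, increments the Killss count on player 0's BP_PlayerShooterCharacter once, then after a delay destroys the weapon and the character.
; If the dead character shares the player's class, it first shows WBP_LoseScreen with that count as score.
; The level-start montage and possession nodes are left unwired.
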(event EventBeginPlay
  ;[1 1 1] Doing a Start level animation
)

(event Collision|EventActorBeginOverlap
  (params (OtherActor :type Actor%20Object%20Reference)))

(event EventTick
  (params (DeltaSeconds :type Float%20%28single-precision%29))
  (if (Class|ShooterChar|IsDead)
    (Utilities|FlowControl|Sequence
      (:then_0
        (Utilities|FlowControl|DoOnce false
          (:Completed
            (bind _asbp_player_shooter_character (Utilities|Casting|CastToBP_PlayerShooterCharacter (Game|GetPlayerCharacter 0)))
            (bind _result (Math|Integer|IncrementInt (Variables|/Game/BP_PlayerShooterCharacter.BP_PlayerShooterCharacter_C|Getkillss _asbp_player_shooter_character))
              (:%20%20
                (bind _output_get (Variables|/Game/BP_PlayerShooterCharacter.BP_PlayerShooterCharacter_C|Setkillss _asbp_player_shooter_character _result)))))))
      (:then_1
        (Utilities|FlowControl|Delay 2.35)
        (Utilities|FlowControl|Sequence
          (:then_0
            (if (== (Utilities|GetClass (Game|GetPlayerCharacter 0)) (Utilities|GetClass self))
              (bind _returnvalue (UserInterface|CreateWidget "/Game/UI/WBP_LoseScreen.WBP_LoseScreen_C" 0 _output_get))
              (UserInterface|Viewport|AddtoViewport _returnvalue 0)))
          (:then_1
            (Actor|DestroyActor (Variables|Default|Getweapon)))
          (:then_2
            (Actor|DestroyActor)))))))

(fn ConstructionScript)