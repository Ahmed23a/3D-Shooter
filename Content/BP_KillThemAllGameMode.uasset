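; BP_KillThemAllGameMode is a game mode that continuously spawns AI shooter characters for a wave-based mode.
; Shortly after BeginPlay, SetupNewWave increments CurrentWave and starts a looping timer that calls SpwanWave by name.
; Each timer tick spawns a BP_ShooterCharacter at a randomly chosen TargetPoint in the level.
; The timer is never cleared here, so spawning has no limit and the wave never advances further.
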(event Custom|SpwanWave
  (CallFunction|SpwanAI))

(event EventBeginPlay
  (Utilities|FlowControl|Delay 2.0)
  (CallFunction|SetupNewWave))

(event EventTick
  (params (DeltaSeconds :type Float%20%28single-precision%29)))

(fn ConstructionScript)

(fn SetupNewWave
  (Math|Integer|IncrementInt (Variables|Default|GetCurrent%20Wave)
    (:%20%20
      (Utilities|Time|SetTimerbyFunctionName 0 "SpwanWave" 1.0 true))))

(fn SpwanAI
  (bind _swpanpoint (CallFunction|GetRandomSpwanPoint))
  (Utilities|IsValid _swpanpoint
    (:Is%20Valid
      (Game|SpawnActorfromClass "/Game/BP_ShooterCharacter.BP_ShooterCharacter_C" (Transformation|GetActorTransform _swpanpoint) "Undefined" 0 0))))

(fn GetRandomSpwanPoint
  (bind _outactors (Actor|GetAllActorsOfClass "/Script/Engine.TargetPoint"))
  (return (Utilities|Array|Get(acopy) _outactors (Math|Random|RandomIntegerinRange 0 (Utilities|Array|LastIndex _outactors)))))