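; Player shooter character Blueprint that adds intro audio, sprint, pause and a lose screen to its parent class.
; Input events change walk speed for sprint (IsSprinting is set inverted) and toggle a lazily created pause widget with matching input mode.
; Tick polls IsDead and creates a lose screen showing the kill count every frame while dead, with no guard.
; Kill counting, death cleanup and start montage are unwired; IncreaseKills is empty.
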(event Custom|CustomEvent)

(event EventBeginPlay
  (|CallParentFunction)
  (Audio|PlaySoundatLocation "/Game/AssetPacks/GameDevTV/VoiceOvers/Intro.Intro" (Transformation|GetActorLocation) "0, 0, 0" 1.0 1.0 0.0 0 0 0))

(event EventTick
  (params (DeltaSeconds :type Float%20%28single-precision%29))
  (if (Class|ShooterChar|IsDead)
    (Utilities|FlowControl|Sequence
      (:then_0
        (bind _returnvalue (UserInterface|CreateWidget "/Game/UI/WBP_LoseScreen.WBP_LoseScreen_C" 0 (Variables|Default|Getkillss)))
        (UserInterface|Viewport|AddtoViewport _returnvalue 0)))))

(event Input|ActionEvents|InputActionPasue
  (params (Key :type Key%20Structure :default "None"))
  (bind _returnvalue (Game|GetPlayerController 0))
  ;[1 1 1] Pause Game / Exist
  (:Pressed
    (Utilities|IsValid (Variables|Default|GetPause%20Menu%20REF)
      (:Is%20Valid
        (if (Game|IsGamePaused)
          (Widget|RemovefromParent (Variables|Default|GetPause%20Menu%20REF))
          (Game|SetGamePaused false)
          (Variables|/Script/Engine.PlayerController|SetbShowMouseCursor _returnvalue false)
          (Input|SetInputModeGameOnly _returnvalue)
          (else
            (UserInterface|Viewport|AddtoViewport (stale _output_get) 0 :!label _label)
            (Game|SetGamePaused true)
            (Variables|/Script/Engine.PlayerController|SetbShowMouseCursor _returnvalue true)
            (Input|SetInputModeGameandUI _returnvalue (Variables|Default|GetPause%20Menu%20REF) "LockInFullscreen" false))))
      (:Is%20Not%20Valid
        (bind _returnvalue_2 (UserInterface|CreateWidget "/Game/UI/WidgetMenus/Pause_Menu.Pause_Menu_C"))
        (bind _output_get (Variables|Default|SetPause%20Menu%20REF _returnvalue_2))
        (goto _label)))))

(event Input|ActionEvents|InputActionSprint
  (params (Key :type Key%20Structure :default "None"))
  ;[1 1 1] Sprint Mechanic
  (:Pressed
    (Variables|Default|SetIs%20Sprinting false)
    (Variables|/Script/Engine.CharacterMovementComponent|SetMaxWalkSpeed (Variables|Character|GetCharacterMovement) 7e+02))
  (:Released
    (Variables|/Script/Engine.CharacterMovementComponent|SetMaxWalkSpeed (Variables|Character|GetCharacterMovement) 3e+02)
    (Variables|Default|SetIs%20Sprinting true)))

(fn ConstructionScript
  (|CallParentFunction))

(fn IncreaseKills)